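; Shop camera actor that handles the slow camera drift and station audio, and also stores the ship upgrade prices.
; BeginPlay gives every upgrade category the same starting price and sets an inflation factor, which is not applied here.
; MoveCamera eases the root backward along X over several seconds, while ResetCamera stops it and snaps to a fixed location.
; Playsound uses a DoOnce to avoid duplicate audio until Stopsound destroys the sound and resets it.
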(event Custom|MoveCamera
  (bind _defaultsceneroot (Variables|Default|GetDefaultSceneRoot))
  (Components|MoveComponentTo _defaultsceneroot (+ (Variables|/Script/Engine.SceneComponent|GetRelativeLocation _defaultsceneroot) "-3000.000000,0.000000,0.000000") (Variables|/Script/Engine.SceneComponent|GetRelativeRotation _defaultsceneroot) true true 8.0 false))

(event Custom|ResetCamera
  (bind _defaultsceneroot (Variables|Default|GetDefaultSceneRoot))
  (Utilities|FlowControl|Sequence
    (:then_0
      (Components|MoveComponentTo _defaultsceneroot (+ (Variables|/Script/Engine.SceneComponent|GetRelativeLocation _defaultsceneroot) "-3000.000000,0.000000,0.000000") (Variables|/Script/Engine.SceneComponent|GetRelativeRotation _defaultsceneroot) true true 8.0 false) ; enters at Stop
    )
    (:then_1
      (Transformation|SetRelativeLocation (Variables|Default|GetDefaultSceneRoot) "-25000.000000,0.000000,50.000000" false false))))

(event Custom|Play%20sound
  (Utilities|FlowControl|DoOnce false
    (:Completed
      (bind _returnvalue (Audio|SpawnSound2D "/Game/Sounds/SoundEffects/SC_ShopStation.SC_ShopStation" 1.0 1.0 0.0 0)))))

(event Custom|Stop%20sound
  (Utilities|IsValid (stale Custom|Play%20sound _returnvalue)
    (:Is%20Valid
      (Audio|Components|Audio|Stop (stale Custom|Play%20sound _returnvalue))
      (Components|DestroyComponent (stale Custom|Play%20sound _returnvalue))
      (Utilities|FlowControl|DoOnce false) ; enters at Reset
    )))

(event EventBeginPlay
  (Variables|Default|SetCargoPriceValue 5e+01)
  (Variables|Default|SetFuelPriceValue 5e+01)
  (Variables|Default|SetShieldPriceValue 5e+01)
  (Variables|Default|SetIntegrityPriceValue 5e+01)
  (Variables|Default|SetTurboPriceValue 5e+01)
  (Variables|Default|SetReactorPriceValue 5e+01)
  (Variables|Default|SetRadarPriceValue 5e+01)
  (Variables|Default|SetOverheatPriceValue 5e+01)
  (Variables|Default|SetFireRatePriceValue 5e+01)
  (Variables|Default|SetLaserPriceValue 5e+01)
  (Variables|Default|SetInflation 1.2))

(event Collision|EventActorBeginOverlap
  (params (OtherActor :type Actor%20Object%20Reference)))

(event EventTick
  (params (DeltaSeconds :type Float%20%28single-precision%29)))

(fn ConstructionScript)