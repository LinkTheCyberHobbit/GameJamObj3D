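; BP_Asteroid is an asteroid hazard that damages the player on contact.
; On BeginPlay it picks a random mesh from an array, and any overlap with its collision sphere spawns a rock explosion.
; Only a BP_Player overlap deals damage, reducing shield first or life once shields are gone, then destroys the asteroid.
; Its IsDestroyed override runs the parent logic and destroys the actor.
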(event OnComponentBeginOverlap(CollisionSphere)
  (params (OverlappedComponent :type Primitive%20Component%20Object%20Reference) (OtherActor :type Actor%20Object%20Reference) (OtherComp :type Primitive%20Component%20Object%20Reference) (OtherBodyIndex :type Integer) (bFromSweep :type Boolean) (SweepResult :type Hit%20Result%20Structure%20%28by%20ref%29))
  (Niagara|SpawnSystematLocation "/Game/NiagaraEffects/NS_RockExplosion.NS_RockExplosion" (Transformation|GetActorLocation))
  (bind _asbp_player (Utilities|Casting|CastToBP_Player OtherActor))
  (if (> (Variables|/Game/Player/BP_Player.BP_Player_C|GetCurrentShield _asbp_player) 0.0)
    (Variables|/Game/Player/BP_Player.BP_Player_C|SetCurrentShield _asbp_player (- (Variables|/Game/Player/BP_Player.BP_Player_C|GetCurrentShield _asbp_player) 2e+01))
    (Default|UpdateShieldVisibility _asbp_player)
    (else
      (Variables|/Game/Player/BP_Player.BP_Player_C|SetCurrentLife _asbp_player (- (Variables|/Game/Player/BP_Player.BP_Player_C|GetCurrentLife _asbp_player) 1e+01))))
  (Actor|DestroyActor))

(event EventBeginPlay
  (|CallParentFunction)
  (Components|StaticMesh|SetStaticMesh (Variables|Default|GetStaticMesh) (.OutItem (Utilities|Array|Random (Variables|Default|GetAsteroidMeshArray)))))

(event EventTick
  (params (DeltaSeconds :type Float%20%28single-precision%29))
  (|CallParentFunction DeltaSeconds))

(fn ConstructionScript
  (|CallParentFunction))

(fn IsDestroyed
  (|CallParentFunction)
  (Actor|DestroyActor))