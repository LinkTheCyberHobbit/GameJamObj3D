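; Spawner actor that fills a box volume with randomly chosen shipwrecks until a target count is reached.
; Tick uses a DoOnce gate reset by a delay to stagger spawns, placing each wreck at a random point with random yaw.
; Each spawn is registered in the player's SpawnedShips list.
; Reset destroys every BP_ShipwreckParent actor, clears that list and zeroes the count, letting spawning resume.
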(event Custom|Reset
  (bind _outactors (Actor|GetAllActorsOfClass "/Game/GameplayObjects/BP_ShipwreckParent.BP_ShipwreckParent_C"))
  (for _array_element _outactors
    (Actor|DestroyActor _array_element))
  (Utilities|Array|Clear (Variables|/Game/Player/BP_Player.BP_Player_C|GetSpawnedShips (Variables|Default|GetAs%20BP%20Player)))
  (Variables|Default|SetNumberSpawned 0))

(event EventBeginPlay
  (bind _asbp_player (Utilities|Casting|CastToBP_Player (Game|GetPlayerCharacter 0)))
  (Variables|Default|SetAs%20BP%20Player _asbp_player))

(event Collision|EventActorBeginOverlap
  (params (OtherActor :type Actor%20Object%20Reference)))

(event EventTick
  (params (DeltaSeconds :type Float%20%28single-precision%29))
  (bind _box (Variables|Default|GetBox))
  (if (< (Variables|Default|GetNumberSpawned) (Variables|Default|GetNumberToSpawn))
    (Utilities|FlowControl|DoOnce false :!label _label
      (:Completed
        (bind _returnvalue (Game|SpawnActorfromClass (.OutItem (Utilities|Array|Random (Variables|Default|GetShipToSpawn))) (Math|Transform|MakeTransform (Math|Random|RandomPointinBoundingBox (Transformation|GetWorldLocation _box) (Components|Box|GetScaledBoxExtent _box)) (Math|Rotator|MakeRotator 0.0 0.0 (.yaw (Math|Random|RandomRotator true))) "1.000000,1.000000,1.000000") "Undefined" "MultiplyWithRoot" 0 0))
        (Utilities|Array|Add (Variables|/Game/Player/BP_Player.BP_Player_C|GetSpawnedShips (Variables|Default|GetAs%20BP%20Player)) _returnvalue)
        (Variables|Default|SetNumberSpawned (+ (Variables|Default|GetNumberSpawned) 1))
        (Utilities|FlowControl|Delay 1.0)
        (goto _label Reset)))))

(fn ConstructionScript)