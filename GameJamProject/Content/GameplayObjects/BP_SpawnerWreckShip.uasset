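; Spawner actor that scatters BP_WreckShip actors inside its Box volume until MaxSpawnable is reached.
; Tick drives a DoOnce gate that spawns one wreck at a random point and yaw, then resets after a random Min–Max delay.
; Each spawn is added to SpawnedArray, whose length sets CurrentSpawned; nothing here removes entries, so the cap counts total spawns.
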(event EventBeginPlay)

(event Collision|EventActorBeginOverlap
  (params (OtherActor :type Actor%20Object%20Reference)))

(event EventTick
  (params (DeltaSeconds :type Float%20%28single-precision%29))
  (bind _box (Variables|Default|GetBox))
  (bind _spawnedarray (Variables|Default|GetSpawnedArray))
  (if (< (Variables|Default|GetCurrentSpawned) (Variables|Default|GetMaxSpawnable))
    (Utilities|FlowControl|DoOnce false :!label _label
      (:Completed
        (bind _returnvalue (Game|SpawnActorfromClass "/Game/GameplayObjects/BP_WreckShip.BP_WreckShip_C" (Math|Transform|MakeTransform (Math|Random|RandomPointinBoundingBox (Transformation|GetWorldLocation _box) (Components|Box|GetScaledBoxExtent _box)) (Math|Rotator|MakeRotator 0.0 0.0 (.yaw (Math|Random|RandomRotator true))) "1.000000,1.000000,1.000000") "Undefined" "MultiplyWithRoot" 0 0))
        (Utilities|Array|Add _spawnedarray _returnvalue)
        (Variables|Default|SetCurrentSpawned (Utilities|Array|Length _spawnedarray))
        (Utilities|FlowControl|Delay (Math|Random|RandomFloatinRange (Variables|Default|GetMin) (Variables|Default|GetMax)))
        (goto _label Reset)))))

(fn ConstructionScript)