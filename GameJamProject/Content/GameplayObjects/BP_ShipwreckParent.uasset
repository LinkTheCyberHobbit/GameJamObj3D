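; Parent Blueprint for salvageable shipwrecks, which the player breaks apart with a laser to gain cargo.
; At BeginPlay it caches the player, the shipwreck spawner and its static mesh components.
; LaserIsHitting uses a DoOnce and short delay to remove random meshes, each adding clamped cargo to the player.
; Once no meshes remain, it updates ship tracking, destroys itself and randomly spawns fuel, a cargo pickup or nothing.
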(event Custom|LaserIsHitting
  (bind _staticmesharray (Variables|Default|GetStaticMeshArray))
  (bind _spawnerref (Variables|Default|GetSpawnerRef))
  (if (> (Utilities|Array|Length _staticmesharray) 0)
    (Utilities|FlowControl|DoOnce false :!label _label
      (:Completed
        (Utilities|FlowControl|Delay 0.1)
        (bind _output_get (Variables|Default|SetActorToDestroy (.OutItem (Utilities|Array|Random _staticmesharray))))
        (Components|DestroyComponent _output_get)
        (Utilities|Array|RemoveItem _staticmesharray _output_get)
        (CallFunction|Salvage)
        (goto _label Reset)))
    (else
      (Utilities|Array|RemoveItem (Variables|/Game/Player/BP_Player.BP_Player_C|GetSpawnedShips (Variables|Default|GetAs%20BP%20Player)) self)
      (Variables|/Game/GameplayObjects/BP_SpawnerShipwreck.BP_SpawnerShipwreck_C|SetNumberSpawned _spawnerref (- (Variables|/Game/GameplayObjects/BP_SpawnerShipwreck.BP_SpawnerShipwreck_C|GetNumberSpawned _spawnerref) 1))
      (Actor|DestroyActor)
      (CallFunction|RandomLoot))))

(event EventBeginPlay
  (bind _asbp_player (Utilities|Casting|CastToBP_Player (Game|GetPlayerCharacter 0)))
  (Variables|Default|SetAs%20BP%20Player _asbp_player)
  (bind _returnvalue (Actor|GetActorOfClass "/Game/GameplayObjects/BP_SpawnerShipwreck.BP_SpawnerShipwreck_C"))
  (Variables|Default|SetSpawnerRef _returnvalue)
  (bind _output_get (Variables|Default|SetStaticMeshArray (Actor|GetComponentsByClass "/Script/Engine.StaticMeshComponent")))
  (for _array_element _output_get
    _))

(event Collision|EventActorBeginOverlap
  (params (OtherActor :type Actor%20Object%20Reference)))

(event EventTick
  (params (DeltaSeconds :type Float%20%28single-precision%29)))

(fn ConstructionScript)

(fn Salvage
  (bind _as_bp_player (Variables|Default|GetAs%20BP%20Player))
  (Variables|/Game/Player/BP_Player.BP_Player_C|SetCurrentCargo _as_bp_player (Math|Float|Clamp(Float) (+ (Variables|/Game/Player/BP_Player.BP_Player_C|GetCurrentCargo _as_bp_player) (Variables|Default|GetCargoAmount)) 0.0 (Variables|/Game/Player/BP_Player.BP_Player_C|GetMaxCargo _as_bp_player))))

(fn RandomLoot
  (bind _returnvalue (Transformation|GetActorLocation))
  (bind _output_get (Variables|Default|SetRandom (Math|Random|RandomIntegerinRange (Variables|Default|GetMin) (Variables|Default|GetMax))))
  (if (== _output_get 1)
    (Game|SpawnActorfromClass "/Game/GameplayObjects/BP_Fuel.BP_Fuel_C" (Math|Transform|MakeTransform _returnvalue "0, 0, 0" "1.000000,1.000000,1.000000") "Undefined" "MultiplyWithRoot" 0 0)
    (Audio|PlaySound2D "/Game/Sounds/SoundEffects/Item.Item" 1.0 1.0 0.0 0 0 :!label _label)
    (elif (== _output_get 2)
      (Game|SpawnActorfromClass "/Game/GameplayObjects/BP_CargoAC.BP_CargoAC_C" (Math|Transform|MakeTransform _returnvalue "0, 0, 0" "1.000000,1.000000,1.000000") "Undefined" "MultiplyWithRoot" 0 0)
      (goto _label))))