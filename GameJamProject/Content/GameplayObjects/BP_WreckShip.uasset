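; BP_WreckShip is a wreck ship game object that grants resources to the player's cargo when destroyed.
; It runs the parent's LaserHit logic every tick.
; Its IsDestroyed override adds RessourceAmount if cargo is below maximum, without clamping the sum.
; It then removes itself from BP_SpawnerWreckShip's SpawnedArray and destroys the actor, even when cargo is full.
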(event EventBeginPlay
  (|CallParentFunction) ; This node is disabled and will not be called.\nDrag off pins to build functionality.
)

(event Collision|EventActorBeginOverlap
  (params (OtherActor :type Actor%20Object%20Reference))
  (|CallParentFunction OtherActor) ; This node is disabled and will not be called.\nDrag off pins to build functionality.
)

(event EventTick
  (params (DeltaSeconds :type Float%20%28single-precision%29))
  (|CallParentFunction DeltaSeconds)
  (CallFunction|LaserHit))

(fn ConstructionScript
  (|CallParentFunction))

(fn IsDestroyed
  (bind _as_bp_player (Variables|Default|GetAs%20BP%20Player))
  (|CallParentFunction)
  (if (< (Variables|/Game/Player/BP_Player.BP_Player_C|GetCurrentCargo _as_bp_player) (Variables|/Game/Player/BP_Player.BP_Player_C|GetMaxCargo _as_bp_player))
    (Variables|/Game/Player/BP_Player.BP_Player_C|SetCurrentCargo _as_bp_player (+ (Variables|/Game/Player/BP_Player.BP_Player_C|GetCurrentCargo _as_bp_player) (Variables|Default|GetRessourceAmount))))
  (bind _returnvalue (Actor|GetActorOfClass "/Game/GameplayObjects/BP_SpawnerWreckShip.BP_SpawnerWreckShip_C"))
  (Utilities|Array|RemoveItem (Variables|/Game/GameplayObjects/BP_SpawnerWreckShip.BP_SpawnerWreckShip_C|GetSpawnedArray _returnvalue) self)
  (Actor|DestroyActor))

(fn LaserHit
  (|CallParentFunction))