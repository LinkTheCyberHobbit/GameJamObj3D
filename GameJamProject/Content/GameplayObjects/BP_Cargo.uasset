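; BP_Cargo is a pickup actor that adds cargo to the player and then destroys itself.
; BeginPlay caches the first player character as BP_Player.
; Any overlap on its Sphere component, with no check on the other actor, raises that player's CurrentCargo by a fixed amount, clamped between zero and MaxCargo.
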(event OnComponentBeginOverlap(Sphere)
  (params (OverlappedComponent :type Primitive%20Component%20Object%20Reference) (OtherActor :type Actor%20Object%20Reference) (OtherComp :type Primitive%20Component%20Object%20Reference) (OtherBodyIndex :type Integer) (bFromSweep :type Boolean) (SweepResult :type Hit%20Result%20Structure%20%28by%20ref%29))
  (bind _as_bp_player (Variables|Default|GetAs%20BP%20Player))
  (Variables|/Game/Player/BP_Player.BP_Player_C|SetCurrentCargo _as_bp_player (Math|Float|Clamp(Float) (+ (Variables|/Game/Player/BP_Player.BP_Player_C|GetCurrentCargo _as_bp_player) 1e+02) 0.0 (Variables|/Game/Player/BP_Player.BP_Player_C|GetMaxCargo _as_bp_player)))
  (Actor|DestroyActor))

(event EventBeginPlay
  (bind _asbp_player (Utilities|Casting|CastToBP_Player (Game|GetPlayerCharacter 0)))
  (Variables|Default|SetAs%20BP%20Player _asbp_player))

(event Collision|EventActorBeginOverlap
  (params (OtherActor :type Actor%20Object%20Reference)))

(event EventTick
  (params (DeltaSeconds :type Float%20%28single-precision%29)))

(fn ConstructionScript)