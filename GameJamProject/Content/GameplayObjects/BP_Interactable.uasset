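; BP_Interactable is an interactable object that shrinks when hit by the player's laser.
; It caches the player character as BP_Player on BeginPlay.
; LaserHit reads the player's hit state and reduces the hit actor's scale by LaserPower, acting on that actor rather than itself.
; Once Z scale is 0.3 or lower, it calls IsDestroyed on the hit actor, which is an empty function here.
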(event EventBeginPlay
  (bind _asbp_player (Utilities|Casting|CastToBP_Player (Game|GetPlayerCharacter 0)))
  (Variables|Default|SetAs%20BP%20Player _asbp_player))

(event EventTick
  (params (DeltaSeconds :type Float%20%28single-precision%29)))

(fn ConstructionScript)

(fn IsDestroyed)

(fn LaserHit
  (bind _as_bp_player (Variables|Default|GetAs%20BP%20Player))
  (bind _hitactor (Variables|/Game/Player/BP_Player.BP_Player_C|GetHitActor _as_bp_player))
  (bind _returnvalue (Transformation|GetActorScale3D _hitactor))
  (if (Variables|/Game/Player/BP_Player.BP_Player_C|GetLaserHit _as_bp_player)
    (if (<= (.z _returnvalue) 0.3)
      (CallFunction|IsDestroyed _hitactor)
      (else
        (Transformation|SetActorScale3D _hitactor (- (Math|Vector|MakeVector (.x _returnvalue) (.y _returnvalue) (.z _returnvalue)) (Variables|/Game/Player/BP_Player.BP_Player_C|GetLaserPower _as_bp_player)))))))